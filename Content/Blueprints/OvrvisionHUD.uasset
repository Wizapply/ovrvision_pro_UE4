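; OvrvisionHUD is a HUD that shows stereo Ovrvision camera images, apparently as an Oculus passthrough view.
; On BeginPlay it opens the Ovrvision device and builds a dynamic OvrvisionOculus material fed by the left and right camera textures.
; DrawHUD updates the camera each frame and draws that material across the whole screen, and EndPlay closes the device.
; The SetOvrvisionSetting function is empty.
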(event `self.ReceiveBeginPlay`
  (`self.OpenOvrvision` 3 0.15)
  (bind _returnvalue (`KismetMaterialLibrary.CreateDynamicMaterialInstance` "/Game/Materials/OvrvisionOculus.OvrvisionOculus"))
  (bind _output_get (set `self.DynamicOvrvisionMaterial` _returnvalue))
  (`MaterialInstanceDynamic.SetTextureParameterValue` _output_get "TextureLeft" (`self.OvrvisionLeftTexture`))
  (`MaterialInstanceDynamic.SetTextureParameterValue` _output_get "TextureRight" (`self.OvrvisionRightTexture`)))

(event `self.ReceiveEndPlay`
  (params (EndPlayReason :type "EEndPlayReason Enum" :default "Destroyed"))
  (`self.CloseOvrvision`))

(event `self.ReceiveDrawHUD`
  (params (SizeX :type Integer) (SizeY :type Integer))
  (`self.UpdateOvrvision`)
  (`self.DrawMaterial` (`self.DynamicOvrvisionMaterial`) 0.0 0.0 (`KismetMathLibrary.Conv_IntToDouble` SizeX) (`KismetMathLibrary.Conv_IntToDouble` SizeY) 1.0 1.0 1.0 1.0 1.0))

(fn `SetOvrvisionSetting`)

(fn `UserConstructionScript`)