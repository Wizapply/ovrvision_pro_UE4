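; Pawn that shows Ovrvision stereo camera passthrough in an HTC Vive headset.
; BeginPlay opens Ovrvision and creates dynamic materials for the left and right eye cubes; EndPlay closes it.
; Each Tick updates Ovrvision and feeds each eye's image into its material as a texture.
; It also repositions both cubes ahead of the player camera from camera and tracked-device transforms, offset sideways by a fixed eye separation.
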(event `self.ReceiveEndPlay`
  (params (EndPlayReason :type "EEndPlayReason Enum" :default "Destroyed"))
  (`OvrvisionBlueprintLibrary.CloseOvrvision`))

(event `self.ReceiveBeginPlay`
  ;[1 1 1] Initialize dynamic material
  (`OvrvisionBlueprintLibrary.OpenOvrvision` 3 0.15)
  (bind _returnvalue (`PrimitiveComponent.CreateDynamicMaterialInstance` (`self.RightCube`) 0 "/Game/Blueprints/Right.Right"))
  (set `self.Right` _returnvalue)
  (bind _returnvalue_2 (`PrimitiveComponent.CreateDynamicMaterialInstance` (`self.LeftCube`) 0 "/Game/Blueprints/Left.Left"))
  (set `self.Left` _returnvalue_2))

(event `self.ReceiveTick`
  (params (DeltaSeconds :type "Float (single-precision)"))
  (bind _returnvalue (`GameplayStatics.GetPlayerCameraManager` 0))
  (bind (_outposition _outorientation) (`SteamVRFunctionLibrary.GetTrackedDevicePositionAndOrientation` 0))
  (bind _returnvalue_2 (`PlayerCameraManager.GetCameraRotation` _returnvalue))
  (bind _returnvalue_3 (`KismetMathLibrary.TransformLocation` (`self.GetTransform` _returnvalue) (`KismetMathLibrary.LessLess_VectorRotator` _outposition _outorientation)))
  (`OvrvisionBlueprintLibrary.UpdateOvrvision`)
  (`MaterialInstanceDynamic.SetTextureParameterValue` (`self.Left`) "Left" (`OvrvisionBlueprintLibrary.GetLeftEye`))
  (`MaterialInstanceDynamic.SetTextureParameterValue` (`self.Right`) "Right" (`OvrvisionBlueprintLibrary.GetRightEye`))
  (`SceneComponent.K2_SetRelativeLocationAndRotation` (`self.LeftCube`) (+ _returnvalue_3 (`KismetMathLibrary.GreaterGreater_VectorRotator` (`KismetMathLibrary.MakeVector` 100.0 (* -1.0 5.0)) _returnvalue_2)) _returnvalue_2 false false)
  (`SceneComponent.K2_SetRelativeLocationAndRotation` (`self.RightCube`) (+ _returnvalue_3 (`KismetMathLibrary.GreaterGreater_VectorRotator` (`KismetMathLibrary.MakeVector` 100.0 5.0) _returnvalue_2)) _returnvalue_2 false false))

(fn `UserConstructionScript`)